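; BP_Trampoline is a platform that bounces the player character when it lands on the Top component.
; A hit with a near-vertical impact normal adds a launch velocity and plays a timeline that stretches Top's X and Y scale.
; The construction script sizes Top and stacks instanced Bottom pieces downward, with their count derived from the BottomEndLength vector's length.
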(event `self.Top.OnComponentHit`
  (params (HitComponent :type "PrimitiveComponent Object Reference") (OtherActor :type "Actor Object Reference") (OtherComp :type "PrimitiveComponent Object Reference") (NormalImpulse :type "Vector Structure") (Hit :type "HitResult Structure (by ref)"))
  (bind _returnvalue (`GameplayStatics.GetPlayerCharacter` 0))
  (if (and (== OtherActor _returnvalue) (== (`.ImpactNormal` (`GameplayStatics.BreakHitResult` Hit)) (0.0 0.0 -0.9) :`ErrorTolerance` 0.1))
    (`Character.LaunchCharacter` _returnvalue (`self.Launch Velocity`) false false)
    (bind (_direction _scale_over_time) (`Timeline|StrechBounce`)
      (:`Update`
        (`SceneComponent.SetWorldScale3D` (`self.Top`) (`KismetMathLibrary.MakeVector` (* (`self.Top_X_Scale`) _scale_over_time) (* (`self.Top_Y_Scale`) _scale_over_time) (`self.Top_Z_Scale`)))))))

(fn `UserConstructionScript`
  (`SceneComponent.SetWorldScale3D` (`self.Top`) (`KismetMathLibrary.MakeVector` (`self.Top_X_Scale`) (`self.Top_Y_Scale`) (`self.Top_Z_Scale`)))
  (for _index (range (+ (`KismetMathLibrary.FTrunc` (/ (`KismetMathLibrary.VSize` (`self.BottomEndLength`)) 100.0)) 1))
    (`InstancedStaticMeshComponent.AddInstance` (`self.Bottom`) (`KismetMathLibrary.MakeTransform` (`KismetMathLibrary.MakeVector` 0.0 0.0 (`KismetMathLibrary.Conv_IntToDouble` (* _index -40)))) false)))